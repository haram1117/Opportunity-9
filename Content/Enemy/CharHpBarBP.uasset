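; CharHpBarBP is an actor that displays a character's health bar, filed under Enemy, through a widget component.
; On BeginPlay it casts the component's widget to CharHpBar and caches its progress bar.
; UpdateLocation moves the actor to a supplied location without sweeping.
; UpdateHpBar sets the bar's percent from Hp divided by MaxHp, converting to float only after the division.
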(event EventBeginPlay
  (bind _aschar_hp_bar (Utilities|Casting|CastToCharHpBar (UserInterface|GetUserWidgetObject (Variables|Default|GetHpBarComp))))
  (Variables|Default|SetProgress%20Bar%20Hp%20Bar (Variables|/Game/Enemy/CharHpBar.CharHpBar_C|GetProgressBarHp _aschar_hp_bar)))

(fn ConstructionScript)

(fn UpdateLocation
  (params (Location :type Vector))
  (Transformation|SetActorLocation Location false false))

(fn UpdateHpBar
  (params (Hp :type Integer) (MaxHp :type Integer))
  (Progress|SetPercent (Variables|Default|GetProgress%20Bar%20Hp%20Bar) (Math|Conversions|ToFloat(Integer) (/ Hp MaxHp))))