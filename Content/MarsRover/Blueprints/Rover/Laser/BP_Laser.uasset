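; BP_Laser is the rover's laser beam actor, which damages enemies and hits resource deposits such as alloy, lithium, iron, perlite and carbon.
; Each Tick it line-traces from the vehicle's beam arrow toward the head camera's aim point and feeds the result to the Niagara beam end.
; A chain of casts on the hit actor calls Damage or Hit every frame.
; StopLaser animates the beam's scale through a timeline, then destroys the actor.
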(event Custom|StopLaser
  (bind _scale (Timeline|StopEffect Play)
    (:Update
      (Effects|Components|ParticleSystem|SetFloatParameter (Variables|Default|GetLaser) "User.Scale" _scale))
    (:Finished
      (Actor|DestroyActor))))

(event EventBeginPlay)

(event EventTick
  (params (DeltaSeconds :type Float%20%28single-precision%29))
  (bind _vehicle (Variables|Default|GetVehicle))
  (bind _headcamera (Variables|/Game/MarsRover/Blueprints/Rover/BP_Vehicle.BP_Vehicle_C|GetHeadCamera _vehicle))
  (Utilities|FlowControl|Sequence
    (:then_0
      (bind _outhit (Collision|LineTraceByChannel (Transformation|GetSocketLocation (Variables|/Game/MarsRover/Blueprints/Rover/BP_Vehicle.BP_Vehicle_C|GetBeamArrow (Variables|Default|GetVehicle)) "None") (+ (Transformation|GetWorldLocation _headcamera) (* (Math|Vector|GetForwardVector (Transformation|GetWorldRotation _headcamera)) (Variables|Default|GetWeapon%20Range))) "TraceTypeQuery1" false (Utilities|Array|MakeArray self) "None"))
      (Effects|Components|ParticleSystem|SetVectorParameter (Variables|Default|GetLaser) "User.BeamEnd" (Math|Vector|SelectVector (.ImpactPoint (Collision|BreakHitResult _outhit)) (.TraceEnd (Collision|BreakHitResult _outhit)) (Utilities|IsValid (.HitActor (Collision|BreakHitResult _outhit)))))
      (bind _asenemy (Utilities|Casting|CastToEnemy (.HitActor (Collision|BreakHitResult _outhit)))
        (:then
          (Default|Damage _asenemy))
        (:CastFailed
          (bind _asbp_alloy (Utilities|Casting|CastToBP_Alloy (.HitActor (Collision|BreakHitResult _outhit)))
            (:then
              (Default|Hit _asbp_alloy))
            (:CastFailed
              (bind _asbp_lithium (Utilities|Casting|CastToBP_Lithium (.HitActor (Collision|BreakHitResult _outhit)))
                (:then
                  (Default|Hit _asbp_lithium))
                (:CastFailed
                  (bind _asbp_iron (Utilities|Casting|CastToBP_Iron (.HitActor (Collision|BreakHitResult _outhit)))
                    (:then
                      (Default|Hit _asbp_iron))
                    (:CastFailed
                      (bind _asbp_perlite (Utilities|Casting|CastToBP_Perlite (.HitActor (Collision|BreakHitResult _outhit)))
                        (:then
                          (Default|Hit _asbp_perlite))
                        (:CastFailed
                          (bind _asbp_carbon (Utilities|Casting|CastToBP_Carbon (.HitActor (Collision|BreakHitResult _outhit)))
                            (:then
                              (Default|Hit _asbp_carbon))
                            (:CastFailed
                              (bind _asbp_carbon_2 (Utilities|Casting|CastToBP_Carbon_2 (.HitActor (Collision|BreakHitResult _outhit))))
                              (Default|Hit _asbp_carbon_2))))))))))))))))

(fn ConstructionScript)